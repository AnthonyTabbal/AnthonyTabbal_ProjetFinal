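; BP_Button is a pressure button that opens a door when a CharacterBP overlaps its Box trigger.
; It lowers Cylinder2 over a second, calls Open on the BP_DOOR found by GetActorOfClass, then waits and raises the cylinder back.
; IsPressed blocks retriggering during the cycle, but it is set before the character cast, so any other overlapping actor leaves the button locked.
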(event OnComponentBeginOverlap(Box)
  (params (OverlappedComponent :type Primitive%20Component%20Object%20Reference) (OtherActor :type Actor%20Object%20Reference) (OtherComp :type Primitive%20Component%20Object%20Reference) (OtherBodyIndex :type Integer) (bFromSweep :type Boolean) (SweepResult :type Hit%20Result%20Structure%20%28by%20ref%29))
  (bind _cylinder2 (Variables|Default|GetCylinder2))
  (bind _cylinder2_2 (Variables|Default|GetCylinder2))
  (bind _returnvalue (Transformation|GetRelativeTransform _cylinder2_2))
  (bind _returnvalue_2 (Transformation|GetRelativeTransform _cylinder2))
  (if (not (Variables|Default|Getis%20pressed))
    (Variables|Default|Setis%20pressed true)
    (Utilities|Casting|CastToCharacterBP OtherActor)
    (Components|MoveComponentTo _cylinder2_2 (- (.location _returnvalue) "0, 0,9.000000") (.rotation _returnvalue) false false 1.0 false)
    (bind _returnvalue_3 (Actor|GetActorOfClass "/Game/BP_DOOR.BP_DOOR_C"))
    (Default|Open _returnvalue_3)
    (Utilities|FlowControl|Delay 1.0)
    (Components|MoveComponentTo _cylinder2 (+ (.location _returnvalue_2) "0, 0,9.000000") (.rotation _returnvalue_2) false false 1.0 false)
    (Variables|Default|Setis%20pressed false)))

(fn ConstructionScript)